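; Game manager actor for a side-scroller that provides the player death routine.
; The construction script adds a GameManager tag to the actor if missing.
; PlayerDeath finds the character by its PlayerChar tag, spawns a sparks effect at its transform and destroys it.
; The event graph does nothing, as its OnDestroyed binding is never executed.
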(event Custom|OnDestroyed_Event_0
  (params (DestroyedActor :type Actor%20Object%20Reference)))

(event EventBeginPlay)

(event Collision|EventActorBeginOverlap
  (params (OtherActor :type Actor%20Object%20Reference)))

(event EventTick
  (params (DeltaSeconds :type Float%20%28single-precision%29)))

(fn ConstructionScript
  (bind _returnvalue (Utilities|String|StringToName "GameManager"))
  (bind _tags (Variables|Actor|GetTags))
  (if (not (Utilities|Array|ContainsItem _tags _returnvalue))
    (Utilities|Array|Add _tags _returnvalue)))

(fn PlayerDeath
  (bind _outactors (Actor|GetAllActorswithTag "PlayerChar"))
  (bind _asside_scroller_character (Utilities|Casting|CastToSideScrollerCharacter (Utilities|Array|Get(acopy) _outactors)))
  (Game|SpawnActorfromClass "/Game/StarterContent/Blueprints/Blueprint_Effect_Sparks.Blueprint_Effect_Sparks_C" (Transformation|GetActorTransform _asside_scroller_character) "Undefined" 0 0)
  (Actor|DestroyActor _asside_scroller_character))